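; AI controller for the Vanguard character that runs its behavior tree and turns perception updates into blackboard data.
; Each perception update traces visibility between stimulus and receiver; an unblocked trace marks the player spotted and alive and stores the position.
; It also starts a timer that later flags stimuli as stale on the blackboard.
; The stale blackboard key is never cleared here, and the dying event is empty.
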(event `self.ReceiveBeginPlay`
  (`self.RunBehaviorTree` "/Game/Characters/mixamoVanguard/vanguardBehaviorTree.vanguardBehaviorTree"))

(event `self.ReceiveTick`
  (params (DeltaSeconds :type "Float (single-precision)")))

(event `self.AIPerception.OnTargetPerceptionUpdated`
  (params (Actor :type "Actor Object Reference") (Stimulus :type "AIStimulus Structure"))
  (bind (_age _expirationage _strength _stimuluslocation _receiverlocation) (break `AIStimulus` Stimulus))
  (bind (_outhits _returnvalue) (`KismetSystemLibrary.LineTraceMulti` _stimuluslocation _receiverlocation "TraceTypeQuery1" false (`|MakeArray` Actor self :!type "Actor Object Reference")))
  (if (not _returnvalue)
    (set `self.LastStimulusLocation` _stimuluslocation)
    (set `self.bStaleStimuli` false)
    (`BlackboardComponent.SetValueAsBool` (`self.Blackboard`) (`self.bPlayerSpotted`) true)
    (`BlackboardComponent.SetValueAsVector` (`self.Blackboard`) (`self.PlayerPositionKey`) (`self.LastStimulusLocation`))
    (`BlackboardComponent.SetValueAsBool` (`self.Blackboard`) "bPlayerAlive" true)
    (`KismetSystemLibrary.K2_SetTimerDelegate` (delegate `ConsiderStimuliStale`) 5.0)))

(event `ConsiderStimuliStale`
  (set `self.bStaleStimuli` true)
  (`BlackboardComponent.SetValueAsBool` (`self.Blackboard`) "bStaleStimuli" true))

(event `Dying_Event`)

(fn `UserConstructionScript`)