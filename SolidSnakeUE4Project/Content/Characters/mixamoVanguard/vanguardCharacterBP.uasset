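; Character Blueprint for the Mixamo Vanguard, handling its death by strangulation.
; On BeginPlay it binds a handler to StartDying, which sets IsBeingStrangled, turns off capsule collision and disables movement and rotation.
; After a fixed delay of several seconds, the handler turns on mesh physics simulation so the body goes limp.
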(event `self.ReceiveBeginPlay`
  (add `self.StartDying` (delegate `EventStartDying`)))

(event `self.ReceiveTick`
  (params (DeltaSeconds :type "Float (single-precision)")))

(event `EventStartDying`
  (bind _charactermovement (`self.CharacterMovement`))
  (set `self.isBeingStrangled` true)
  (`PrimitiveComponent.SetCollisionEnabled` (`self.CapsuleComponent`) "NoCollision")
  (`CharacterMovementComponent.DisableMovement` _charactermovement)
  (set `CharacterMovementComponent.bOrientRotationToMovement` false _charactermovement)
  (set `CharacterMovementComponent.RotationRate` (struct) _charactermovement)
  (`KismetSystemLibrary.Delay` 7.2)
  (`PrimitiveComponent.SetSimulatePhysics` (`self.Mesh`) true))

(fn `UserConstructionScript`)