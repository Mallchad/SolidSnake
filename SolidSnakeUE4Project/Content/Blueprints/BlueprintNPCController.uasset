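; AI controller for the Vanguard character NPC that chases the last location reported by AI perception until the pawn starts dying.
; Each tick, ChasePlayer re-paths to a random reachable point near that stimulus when enough time or target movement has accumulated.
; The give-up check subtracts current time from stimulus time, so it stays true for any positive limit.
; The looping AI timer event is empty, and the stale-stimulus flag is never read.
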(event `self.ReceiveBeginPlay`
  (bind _asvanguard_character_bp (cast `/Game/Characters/mixamoVanguard/vanguardCharacterBP` (`self.K2_GetPawn` self))
    (:`then`
      (set `self.ControlledPawn` _asvanguard_character_bp)
      (add `/Game/Characters/mixamoVanguard/vanguardCharacterBP.StartDying` (`self.ControlledPawn`) (delegate `StartDying`))
      (`KismetSystemLibrary.K2_SetTimerDelegate` (delegate `EventAITick`) (/ 1.0 (`self.PerceptionUpdateRate`)) true))
    (:`CastFailed`
      (`KismetSystemLibrary.PrintText` "Cast failed, bind event will fail" false))))

(event `self.ReceivePossess`
  (params (PossessedPawn :type "Pawn Object Reference")))

(event `EventAITick`)

(event `self.ReceiveTick`
  (params (DeltaSeconds :type "Float (single-precision)"))
  (if (not (`self.bDying`))
    (`self.ChasePlayer` (`self.LastStimulusLocation`))))

(event `self.AIPerception.OnTargetPerceptionUpdated`
  (params (Actor :type "Actor Object Reference") (Stimulus :type "AIStimulus Structure"))
  (set `self.LastStimulus` Stimulus)
  (if (not (`self.bDying`))
    (set `self.LastStimulusTime` (`self.GetGameTimeSinceCreation`))
    (set `self.LastStimulusLocation` (`.StimulusLocation` (break `AIStimulus` (`self.LastStimulus`))))
    (set `self.bStaleStimuli` false)
    (`KismetSystemLibrary.K2_SetTimerDelegate` (delegate `ConsiderStimuliStale`) 5.0)))

(event `ConsiderStimuliStale`
  (set `self.bStaleStimuli` true))

(event `StartDying`
  (set `self.bDying` true))

(fn `ChasePlayer`
  (params (StimulusLocation :type "Vector Structure"))
  (if (and (or (> (- (`self.GetGameTimeSinceCreation`) (`self.LastNavUpdateTime`)) (`self.StaleStimulusSeconds`)) (> (`KismetMathLibrary.Vector_Distance` (`local.StimulusLocation`) (`self.NavTarget`)) (`self.StaleStimulusDistance`))) (< (- (`self.LastStimulusTime`) (`self.GetGameTimeSinceCreation`)) (`self.GiveUpChaseSeconds`)))
    (`self.MoveToLocation` self (`NavigationSystemV1.K2_GetRandomReachablePointInRadius` (`local.StimulusLocation`) (`self.RandomReachableRadius`) null null) (`CapsuleComponent.GetScaledCapsuleRadius` (`Character.CapsuleComponent` (`self.ControlledPawn`))) true true false true true)
    (set `self.NavTarget` (`.StimulusLocation` (break `AIStimulus` (`self.LastStimulus`))))
    (set `self.LastNavUpdateTime` (`self.GetGameTimeSinceCreation`))))

(fn `UserConstructionScript`)